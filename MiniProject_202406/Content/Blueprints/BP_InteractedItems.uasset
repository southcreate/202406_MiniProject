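; BP_InteractedItems is a data-driven interactable item whose mesh, scale and name come from its DT_Items row in the construction script.
; On BeginPlay each item creates its own hidden WBP_Interaction widget and passes itself to it.
; SetWidgetVisibility shows or hides that widget, and a binding on BP_FPCharacter lets the character trigger its removal from the viewport.
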(event `self.ReceiveBeginPlay`
  (bind _returnvalue (`|CreateWidget` "/Game/Blueprints/Widgets/WBP_Interaction.WBP_Interaction_C" (`GameplayStatics.GetPlayerController` 0)))
  (bind _output_get (set `self.WidgetReference` _returnvalue))
  (`/Game/Blueprints/Widgets/WBP_Interaction.Get BP_InteractedItem` _returnvalue self)
  (`UserWidget.AddToViewport` _output_get 0)
  (`Widget.SetVisibility` _output_get "Hidden")
  (bind _asbp_fpcharacter (cast `/Game/Blueprints/BP_FPCharacter` (`GameplayStatics.GetPlayerCharacter` 0)))
  (add `/Game/Blueprints/BP_FPCharacter.DeleteWidget` _asbp_fpcharacter (delegate `Delete Widget`)))

(event `Delete Widget`
  (bind _widgetreference (`self.WidgetReference`))
  (`/Engine/EditorBlueprintResources/StandardMacros.IsValid` _widgetreference
    (:`Is Valid`
      (`Widget.RemoveFromParent` _widgetreference))))

(event `self.InteractionCollision.OnComponentHit`
  (params (HitComponent :type "PrimitiveComponent Object Reference") (OtherActor :type "Actor Object Reference") (OtherComp :type "PrimitiveComponent Object Reference") (NormalImpulse :type "Vector Structure") (Hit :type "HitResult Structure (by ref)")))

(fn `Set Widget Visibility`
  (params (Visible :type Boolean))
  (bind _widgetreference (`self.WidgetReference`))
  (if Visible
    (`/Engine/EditorBlueprintResources/StandardMacros.IsValid` _widgetreference
      (:`Is Valid`
        (`Widget.SetVisibility` _widgetreference "Visible")))
    (else
      (`/Engine/EditorBlueprintResources/StandardMacros.IsValid` _widgetreference
        (:`Is Valid`
          (`Widget.SetVisibility` _widgetreference "Hidden"))))))

(fn `UserConstructionScript`
  (bind _staticmesh (`self.StaticMesh`))
  (bind _returnvalue (`|GetDataTableRow` "/Game/DataTables/DT_Items.DT_Items" (`self.RowName`))
    (:`then`
      (bind (_itemname _staticmesh_2 _itemsize) (break `/Game/DataTables/ST_Items` _returnvalue))
      (`StaticMeshComponent.SetStaticMesh` _staticmesh _staticmesh_2)
      (`SceneComponent.SetRelativeScale3D` _staticmesh (* _itemsize (`SceneComponent.K2_GetComponentScale` _staticmesh)))
      (set `self.Item NameVar` _itemname))))