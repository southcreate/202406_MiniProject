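; BP_TestCamera is a player-controlled test camera, moved and rotated through Enhanced Input.
; BeginPlay adds the IMC_TestCam mapping context through BP_PlayerController.
; Move input is scaled by speed and frame delta time, then passed to MoveForward and MoveRight.
; Look input applies sensitivity-scaled pitch and yaw as local rotation on the Camera, only while the right mouse button is held.
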(event `self.ReceiveBeginPlay`
  (bind _asbp_player_controller (cast `/Game/Blueprints/BP_PlayerController` (`self.GetController`)))
  (`EnhancedInputSubsystemInterface.AddMappingContext` (pcsubsystem `EnhancedInputLocalPlayerSubsystem` _asbp_player_controller) "/Game/Blueprints/IMC_TestCam.IMC_TestCam" 0 (struct)))

(event `EnhancedInput|/Game/Blueprints/IA_CamMove`
  (params (ActionValue :type "Vector2D Structure") (ElapsedSeconds :type "Float (double-precision)") (TriggeredSeconds :type "Float (double-precision)") (InputAction :type "InputAction Object Reference" :default "/Game/Blueprints/IA_CamMove.IA_CamMove"))
  (bind (_returnvalue_x _returnvalue_y) (`KismetMathLibrary.BreakVector2D` (* ActionValue (* (`self.MoveSpeed`) (`GameplayStatics.GetWorldDeltaSeconds`)))))
  (:`Triggered`
    (`self.MoveForward` _returnvalue_x)
    (`self.MoveRight` _returnvalue_y)))

(event `EnhancedInput|/Game/Blueprints/IA_CamLook`
  (params (ActionValue :type "Vector2D Structure") (ElapsedSeconds :type "Float (double-precision)") (TriggeredSeconds :type "Float (double-precision)") (InputAction :type "InputAction Object Reference" :default "/Game/Blueprints/IA_CamLook.IA_CamLook"))
  (bind (_x _y) (`KismetMathLibrary.BreakVector2D` ActionValue))
  (bind _mousesensitivity (`self.MouseSensitivity`))
  (bind (_returnvalue_roll _returnvalue_pitch) (`KismetMathLibrary.BreakRotator` (`KismetMathLibrary.MakeRotator` 0.0 (* _y _mousesensitivity))))
  (bind (_returnvalue_roll_2 _returnvalue_pitch_2 _returnvalue_yaw) (`KismetMathLibrary.BreakRotator` (`KismetMathLibrary.MakeRotator` 0.0 0.0 (* _x _mousesensitivity))))
  (:`Triggered`
    (if (stale `Key|RightMouseButton` _output_get)
      (`SceneComponent.K2_AddLocalRotation` (`self.Camera`) (`KismetMathLibrary.MakeRotator` 0.0 _returnvalue_pitch _returnvalue_yaw) false false))))

(event `Key|RightMouseButton`
  (params (Key :type "Key Structure"))
  (:`Pressed`
    (bind _output_get (set `self.bMouseClicked` true)))
  (:`Released`
    (set `self.bMouseClicked` false)))

(fn `UserConstructionScript`)