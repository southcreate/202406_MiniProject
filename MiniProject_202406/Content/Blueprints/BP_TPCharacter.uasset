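; Third-person player character that handles look and movement through Enhanced Input.
; On BeginPlay it adds the IMC_TP_Basic mapping context through BP_PlayerController and caches the movement component's max speed.
; Look actions drive controller yaw and pitch scaled by MouseSensitivity.
; Move input follows ThirdPersonCam's right and forward vectors, scaled by cached max speed and frame delta time.
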(event `self.ReceiveBeginPlay`
  (bind _asbp_player_controller (cast `/Game/Blueprints/BP_PlayerController` (`self.GetController`)))
  (`EnhancedInputSubsystemInterface.AddMappingContext` (pcsubsystem `EnhancedInputLocalPlayerSubsystem` _asbp_player_controller) "/Game/Input/ThirdPersonInputs/IMC_TP_Basic.IMC_TP_Basic" 0 (struct))
  (set `self.MaxSpeed` (`MovementComponent.GetMaxSpeed` (`self.CharacterMovement`))))

(event `EnhancedInput|/Game/Input/ThirdPersonInputs/IA_TP_LookRight`
  (params (ActionValue :type "Float (double-precision)") (ElapsedSeconds :type "Float (double-precision)") (TriggeredSeconds :type "Float (double-precision)") (InputAction :type "InputAction Object Reference" :default "/Game/Input/ThirdPersonInputs/IA_TP_LookRight.IA_TP_LookRight"))
  (:`Triggered`
    (`self.AddControllerYawInput` (* (`self.MouseSensitivity`) ActionValue))))

(event `EnhancedInput|/Game/Input/ThirdPersonInputs/IA_TP_LookUp`
  (params (ActionValue :type "Float (double-precision)") (ElapsedSeconds :type "Float (double-precision)") (TriggeredSeconds :type "Float (double-precision)") (InputAction :type "InputAction Object Reference" :default "/Game/Input/ThirdPersonInputs/IA_TP_LookUp.IA_TP_LookUp"))
  (:`Triggered`
    (`self.AddControllerPitchInput` (* (`self.MouseSensitivity`) ActionValue))))

(event `EnhancedInput|/Game/Input/ThirdPersonInputs/IA_TP_Move`
  (params (ActionValue :type "Vector2D Structure") (ElapsedSeconds :type "Float (double-precision)") (TriggeredSeconds :type "Float (double-precision)") (InputAction :type "InputAction Object Reference" :default "/Game/Input/ThirdPersonInputs/IA_TP_Move.IA_TP_Move"))
  (bind (_x _y) (`KismetMathLibrary.BreakVector2D` ActionValue))
  (bind _thirdpersoncam (`self.ThirdPersonCam`))
  (bind _returnvalue (* (`self.MaxSpeed`) (`GameplayStatics.GetWorldDeltaSeconds`)))
  (:`Triggered`
    (`self.AddMovementInput` (`SceneComponent.GetRightVector` _thirdpersoncam) (* _x _returnvalue))
    (`self.AddMovementInput` (`SceneComponent.GetForwardVector` _thirdpersoncam) (* _y _returnvalue))))

(fn `UserConstructionScript`)