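; First-person player character Blueprint that handles walking, mouse look and jumping through Enhanced Input.
; BeginPlay adds the character mapping context to the player controller and caches max movement speed.
; Move input is scaled by that speed and frame delta along actor forward and right, setting a backward-walk flag; look input is scaled by mouse sensitivity.
; Jump raises the max jump count after jumping, allowing repeated mid-air jumps.
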(event `self.ReceiveBeginPlay`
  (bind _asbp_player_controller (cast `/Game/Blueprints/BP_PlayerController` (`self.GetController`)))
  (`EnhancedInputSubsystemInterface.AddMappingContext` (pcsubsystem `EnhancedInputLocalPlayerSubsystem` _asbp_player_controller) "/Game/Input/Character/IMC_Character.IMC_Character" 0 (struct))
  (set `self.MaxSpeed` (`MovementComponent.GetMaxSpeed` (`self.CharacterMovement`))))

(event `EnhancedInput|/Game/Input/Character/IA_Move`
  (params (ActionValue :type "Vector2D Structure") (ElapsedSeconds :type "Float (double-precision)") (TriggeredSeconds :type "Float (double-precision)") (InputAction :type "InputAction Object Reference" :default "/Game/Input/Character/IA_Move.IA_Move"))
  (bind (_x _y) (`KismetMathLibrary.BreakVector2D` ActionValue))
  (bind _returnvalue (* (`self.MaxSpeed`) (`GameplayStatics.GetWorldDeltaSeconds`)))
  (bind _returnvalue_2 (* _x _returnvalue))
  (:`Triggered`
    (`self.AddMovementInput` (`self.GetActorForwardVector`) _returnvalue_2)
    (`self.AddMovementInput` (`self.GetActorRightVector`) (* _y _returnvalue))
    (if (< _returnvalue_2 0.0)
      (set `self.bIsWalkBackward` true)
      (else
        (set `self.bIsWalkBackward` false)))))

(event `EnhancedInput|/Game/Input/Character/IA_LookRight`
  (params (ActionValue :type "Float (double-precision)") (ElapsedSeconds :type "Float (double-precision)") (TriggeredSeconds :type "Float (double-precision)") (InputAction :type "InputAction Object Reference" :default "/Game/Input/Character/IA_LookRight.IA_LookRight"))
  (:`Triggered`
    (`self.AddControllerYawInput` (* ActionValue (`self.MouseSensitivity`)))))

(event `EnhancedInput|/Game/Input/Character/IA_LookUP`
  (params (ActionValue :type "Float (double-precision)") (ElapsedSeconds :type "Float (double-precision)") (TriggeredSeconds :type "Float (double-precision)") (InputAction :type "InputAction Object Reference" :default "/Game/Input/Character/IA_LookUP.IA_LookUP"))
  (:`Triggered`
    (`self.AddControllerPitchInput` (* (`self.MouseSensitivity`) ActionValue))))

(event `EnhancedInput|/Game/Input/Character/IA_Jump`
  (params (ActionValue :type Boolean) (ElapsedSeconds :type "Float (double-precision)") (TriggeredSeconds :type "Float (double-precision)") (InputAction :type "InputAction Object Reference" :default "/Game/Input/Character/IA_Jump.IA_Jump"))
  (:`Triggered`
    (if ActionValue
      (`self.Jump`)
      (set `self.JumpMaxCount` 100))))

(fn `UserConstructionScript`)