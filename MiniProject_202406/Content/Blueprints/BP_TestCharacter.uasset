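; BP_TestCharacter is a test player character with Enhanced Input movement and look controls.
; On BeginPlay it adds IMC_Character through BP_PlayerController's input subsystem and caches the movement component's max speed.
; Move input feeds CharacterMovement's input vector directly on world X/Y, scaled by max speed and delta time, independent of view direction.
; Look input drives controller yaw and pitch.
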(event `self.ReceiveBeginPlay`
  (bind _asbp_player_controller (cast `/Game/Blueprints/BP_PlayerController` (`self.GetController`)))
  (`EnhancedInputSubsystemInterface.AddMappingContext` (pcsubsystem `EnhancedInputLocalPlayerSubsystem` _asbp_player_controller) "/Game/Input/IMC_Character.IMC_Character" 0 (struct))
  (set `self.MaxSpeed` (`MovementComponent.GetMaxSpeed` (`self.CharacterMovement`))))

(event `EnhancedInput|/Game/Input/IA_CharacterMove`
  (params (ActionValue :type "Vector2D Structure") (ElapsedSeconds :type "Float (double-precision)") (TriggeredSeconds :type "Float (double-precision)") (InputAction :type "InputAction Object Reference" :default "/Game/Input/IA_CharacterMove.IA_CharacterMove"))
  (bind (_x _y) (`KismetMathLibrary.BreakVector2D` ActionValue))
  (bind _returnvalue (* (`self.MaxSpeed`) (`GameplayStatics.GetWorldDeltaSeconds`)))
  (:`Triggered`
    (`PawnMovementComponent.AddInputVector` (`self.CharacterMovement`) (`KismetMathLibrary.MakeVector` (* _x _returnvalue) (* _y _returnvalue)) false)))

(event `EnhancedInput|/Game/Input/IA_CharacterLook`
  (params (ActionValue :type "Vector2D Structure") (ElapsedSeconds :type "Float (double-precision)") (TriggeredSeconds :type "Float (double-precision)") (InputAction :type "InputAction Object Reference" :default "/Game/Input/IA_CharacterLook.IA_CharacterLook"))
  (bind (_x _y) (`KismetMathLibrary.BreakVector2D` ActionValue))
  (:`Triggered`
    (`self.AddControllerYawInput` _x)
    (`self.AddControllerPitchInput` _y)))

(fn `UserConstructionScript`)