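; BP_FreeCam is a free-fly camera pawn, controlled through the IMC_TestCam input mapping context that it adds on BeginPlay.
; Enhanced Input look actions apply sensitivity-scaled yaw and pitch to the controller.
; Move input offsets the location along the actor's forward and right vectors, scaled by speed and delta time, without sweeping for collision.
; The mouse wheel steps movement speed up or down within loosely checked limits.
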(event `self.ReceiveBeginPlay`
  (bind _asbp_player_controller (cast `/Game/Blueprints/BP_PlayerController` (`self.GetController`)))
  (`EnhancedInputSubsystemInterface.AddMappingContext` (pcsubsystem `EnhancedInputLocalPlayerSubsystem` _asbp_player_controller) "/Game/Input/Camera/IMC_TestCam.IMC_TestCam" 0 (struct)))

(event `EnhancedInput|/Game/Input/Camera/IA_Cam_LookRight`
  (params (ActionValue :type "Float (double-precision)") (ElapsedSeconds :type "Float (double-precision)") (TriggeredSeconds :type "Float (double-precision)") (InputAction :type "InputAction Object Reference" :default "/Game/Input/Camera/IA_Cam_LookRight.IA_Cam_LookRight"))
  (:`Triggered`
    (`self.AddControllerYawInput` (* ActionValue (`self.MouseSensitivity`)))))

(event `EnhancedInput|/Game/Input/Camera/IA_Cam_LookUp`
  (params (ActionValue :type "Float (double-precision)") (ElapsedSeconds :type "Float (double-precision)") (TriggeredSeconds :type "Float (double-precision)") (InputAction :type "InputAction Object Reference" :default "/Game/Input/Camera/IA_Cam_LookUp.IA_Cam_LookUp"))
  (:`Triggered`
    (`self.AddControllerPitchInput` (* (`self.MouseSensitivity`) ActionValue))))

(event `EnhancedInput|/Game/Input/Camera/IA_Cam_Move`
  (params (ActionValue :type "Vector2D Structure") (ElapsedSeconds :type "Float (double-precision)") (TriggeredSeconds :type "Float (double-precision)") (InputAction :type "InputAction Object Reference" :default "/Game/Input/Camera/IA_Cam_Move.IA_Cam_Move"))
  (bind (_x _y) (`KismetMathLibrary.BreakVector2D` ActionValue))
  (bind _returnvalue (* (`self.CamMoveSpeed`) (`GameplayStatics.GetWorldDeltaSeconds`)))
  (:`Triggered`
    (`self.K2_SetActorLocation` (+ (`self.K2_GetActorLocation`) (* (`self.GetActorRightVector`) (* _x _returnvalue)) (* (* _y _returnvalue) (`self.GetActorForwardVector`))))))

(event `Key|MouseScrollUp`
  (params (Key :type "Key Structure"))
  (bind _cammovespeed (`self.CamMoveSpeed`))
  (:`Pressed`
    (if (not (> _cammovespeed 1000.0))
      (set `self.CamMoveSpeed` (+ _cammovespeed 50.0)))))

(event `Key|MouseScrollDown`
  (params (Key :type "Key Structure"))
  (bind _cammovespeed (`self.CamMoveSpeed`))
  (:`Pressed`
    (if (not (< _cammovespeed 1.0))
      (set `self.CamMoveSpeed` (- _cammovespeed 50.0)))))

(fn `UserConstructionScript`)